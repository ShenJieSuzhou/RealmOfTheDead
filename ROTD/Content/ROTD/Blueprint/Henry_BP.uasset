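; Henry_BP is the first-person player character, handling sprint, aiming, firing, weapon switching and dropping, healing, flashlight and health.
; A looping timer drives camera line traces that use an interface to show pickup or door prompts for inventory and use actions.
; Shotgun reload chains start, loop and stop montages per shell, while movement emits pawn noise each tick.
; Damage pulses a material-collection vignette, and death spawns a body and shifts the camera.
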(event `self.ReceiveBeginPlay`
  (bind _returnvalue (`GameplayStatics.GetPlayerController` 0))
  (bind _maxhealth (`self.MaxHealth`))
  ;[1 1 1] Begin play
  (bind _output_get (set `self.CurrentHealth` _maxhealth))
  (`self.UpdatePlayerHealth` _output_get _maxhealth)
  (`WidgetBlueprintLibrary.SetInputMode_GameOnly` _returnvalue)
  (set `PlayerController.bShowMouseCursor` false _returnvalue)
  (`self.Set Interact System`))

(event `self.ReceiveTick`
  (params (DeltaSeconds :type "Float (single-precision)"))
  (`self.Sound`))

(event `InputAction|SpeedUp`
  (params (Key :type "Key Structure"))
  (bind _charactermovement (`self.CharacterMovement`))
  ;[1 1 1] Speed Up
  (:`Pressed`
    (set `CharacterMovementComponent.MaxWalkSpeed` 500.0 _charactermovement)
    (set `self.IsRunning` true))
  (:`Released`
    (set `CharacterMovementComponent.MaxWalkSpeed` 375.0 _charactermovement)
    (set `self.IsRunning` false)))

(event `InputAction|Reload`
  (params (Key :type "Key Structure"))
  ;[1 1 1] Reload And Fire
  (:`Pressed`
    (`self.Reload`)))

(event `StopReload`
  ;[1 1 1] Reload And Fire
  (bind _returnvalue (`AnimInstance.Montage_Play` (`SkeletalMeshComponent.GetAnimInstance` (`self.Mesh1P`)) "/Game/ROTD/Arms/Animations/CHANM_FP-Arms_SHTG_870-AC-ReloadStop_Montage.CHANM_FP-Arms_SHTG_870-AC-ReloadStop_Montage" 1.0 "MontageLength" 0.0 true))
  (`AnimInstance.Montage_Play` (`SkeletalMeshComponent.GetAnimInstance` (`WeaponPickup.FP_Gun` (`self.CurrentWeapon`))) "/Game/ROTD/Arms/WeaponsAnimation/Anim_FP-Arms_SHTG_870-AC-ReloadStop_Montage.Anim_FP-Arms_SHTG_870-AC-ReloadStop_Montage" 1.0 "MontageLength" 0.0 true)
  (`KismetSystemLibrary.Delay` _returnvalue)
  (set `self.IsReloading` false))

(event `LoopReload`
  (bind _currentweapon (`self.CurrentWeapon`))
  ;[1 1 1] Reload And Fire
  (bind _returnvalue (`AnimInstance.Montage_Play` (`SkeletalMeshComponent.GetAnimInstance` (`self.Mesh1P`)) "/Game/ROTD/Arms/Animations/CHANM_FP-Arms_SHTG_870-AC-ReloadLoop_Montage.CHANM_FP-Arms_SHTG_870-AC-ReloadLoop_Montage" 1.0 "MontageLength" 0.0 true))
  (`AnimInstance.Montage_Play` (`SkeletalMeshComponent.GetAnimInstance` (`WeaponPickup.FP_Gun` (`self.CurrentWeapon`))) "/Game/ROTD/Arms/WeaponsAnimation/Anim_FP-Arms_SHTG_870-AC-ReloadLoop_Montage.Anim_FP-Arms_SHTG_870-AC-ReloadLoop_Montage" 1.0 "MontageLength" 0.0 true)
  (`KismetSystemLibrary.Delay` _returnvalue)
  (bind _result (`/Engine/EditorBlueprintResources/StandardMacros.IncrementInt` (`WeaponPickup.MagazineBullets` _currentweapon))
    (:`  `
      (if (or (`self.StopReloading`) (>= _result (`WeaponPickup.MaxAmmoCount` _currentweapon)))
        (`self.StopReload`)
        (else
          (`self.LoopReload`))))))

(event `self.ShotgunReload`
  ;[1 1 1] Reload And Fire
  (bind _returnvalue (`AnimInstance.Montage_Play` (`SkeletalMeshComponent.GetAnimInstance` (`self.Mesh1P`)) "/Game/ROTD/Arms/Animations/CHANM_FP-Arms_SHTG_870-AC-ReloadStart_Montage.CHANM_FP-Arms_SHTG_870-AC-ReloadStart_Montage" 1.0 "MontageLength" 0.0 true))
  (`AnimInstance.Montage_Play` (`SkeletalMeshComponent.GetAnimInstance` (`WeaponPickup.FP_Gun` (`self.CurrentWeapon`))) "/Game/ROTD/Arms/WeaponsAnimation/Anim_FP-Arms_SHTG_870-AC-ReloadStart_Montage.Anim_FP-Arms_SHTG_870-AC-ReloadStart_Montage" 1.0 "MontageLength" 0.0 true)
  (`KismetSystemLibrary.Delay` _returnvalue)
  (if (`self.StopReloading`)
    (`self.StopReload`)
    (else
      (`self.LoopReload`))))

(event `InputAction|ArmDown`
  (params (Key :type "Key Structure"))
  (bind _weapontype (`self.WeaponType`))
  (bind _returnvalue (or (== _weapontype 0) (== _weapontype 1)))
  ;[1 1 1] AimDown
  (:`Pressed`
    (set `self.IsAiming` true)
    (if (not _returnvalue)
      (`self.OnAimDownSight`)
      (bind (_direction _float) (`Timeline|Timeline_0` :!via `PlayFromStart`)
        (:`Update`
          (set `self.ADSDistance` 60.0)
          (`CameraComponent.SetFieldOfView` (`self.FirstPersonCameraComponent`) (`KismetMathLibrary.Lerp` 90.0 (`self.ADSDistance`) _float))
          (`SceneComponent.K2_SetRelativeTransform` (`self.Mesh`) (`KismetMathLibrary.MakeTransform` (`KismetMathLibrary.VLerp` (3.177 -1.02 -23.0) (3.177 0.0 -16.0) _float) (struct :`Yaw` -1.0)) false false)))))
  (:`Released`
    (set `self.IsAiming` false)
    (if (not _returnvalue)
      (`self.OnRecoverAimDownSight`)
      (bind (_direction_2 _float_2) (`Timeline|Timeline_1` :!via `PlayFromStart`)
        (:`Update`
          (`CameraComponent.SetFieldOfView` (`self.FirstPersonCameraComponent`) (`KismetMathLibrary.Lerp` (`self.ADSDistance`) 90.0 _float_2))
          (`SceneComponent.K2_SetRelativeTransform` (`self.Mesh`) (`KismetMathLibrary.MakeTransform` (`KismetMathLibrary.VLerp` (3.177 -0.0 -16.0) (3.177 -1.02 -23.0) _float_2) (struct :`Yaw` 4.0)) false false))))))

(event `InputAction|Fire`
  (params (Key :type "Key Structure"))
  (bind _returnvalue (== (`self.WeaponType`) 0))
  ;[1 1 1] Reload And Fire
  (:`Pressed`
    (if _returnvalue
      (`|PlayMontage` (`self.Mesh1P`) "/Game/ROTD/Arms/Animations/Anim_Hands_Empty_Dukes_Attack_01_Montage.Anim_Hands_Empty_Dukes_Attack_01_Montage")
      (else
        (`self.OnFire`))))
  (:`Released`
    (if (not _returnvalue)
      (`self.OnStopFire`))))

(event `InputAction|GM`
  (params (Key :type "Key Structure"))
  ;[1 1 1] GM
)

(event `UnderAttack`
  (params (DamageNum :type "Float (double-precision)"))
  (bind _maxhealth (`self.MaxHealth`))
  (bind _charactermovement (`self.CharacterMovement`))
  (bind _returnvalue (- (`self.CurrentHealth`) DamageNum))
  ;[1 1 1] PlayerUnderAttack
  (if (<= _returnvalue 0.0)
    (set `self.IsDead` true)
    (`self.UpdatePlayerHealth` 0.0 _maxhealth)
    (`MovementComponent.StopMovementImmediately` _charactermovement)
    (set `CharacterMovementComponent.MaxWalkSpeed` 0.0 _charactermovement)
    (`self.ShowDeath`)
    (else
      (bind _output_get (set `self.CurrentHealth` _returnvalue))
      (`self.UpdatePlayerHealth` _output_get _maxhealth)
      (bind (_direction _float) (`Timeline|Veginette` :!via `PlayFromStart`)
        (:`Update`
          (`KismetMaterialLibrary.SetScalarParameterValue` "/Game/ROTD/Material/FPSMaterial_MPC.FPSMaterial_MPC" "VignetteAmount" _float))))))

(event `OnInteractSystem`
  ;[1 1 1] InteractSys
  (bind (_ishit _hitactor) (`self.EyeSightLineTrace`))
  (if _ishit
    (bind _output_get (set `self.Hit Actor` _hitactor))
    (bind _result (`self.Can Display Interact Tips` _output_get))
    (if _result
      (bind _output_get_2 (set `self.Looking at Actor` (`self.Hit Actor`)))
      (`self.Show Interactive Info` _output_get_2)
      (else
        (`self.HideInteractiveInfo` _output_get_2)))
    (elif (`KismetSystemLibrary.IsValid` (`self.Looking at Actor`))
      (bind _result_2 (`self.Can Display Interact Tips` null))
      (if _result_2
        (`self.HideInteractiveInfo` (`self.Looking at Actor`))))))

(event `ShowDeath`
  (bind _returnvalue (`self.GetTransform`))
  ;[1 1 1] PlayerUnderAttack
  (bind _ashenry_bp (cast `/Game/ROTD/Blueprint/Henry_BP` (`GameplayStatics.GetPlayerCharacter` 0)))
  (`self.PlayerDieAndHideCross` _ashenry_bp)
  (`SceneComponent.SetVisibility` (`self.Mesh1P`) false false)
  (`/Engine/EditorBlueprintResources/StandardMacros.DoOnce` false
    (:`Completed`
      (bind _returnvalue_2 (`|SpawnActorFromClass` "/Game/ROTD/Blueprint/HenryDy_BP.HenryDy_BP_C" (`KismetMathLibrary.MakeTransform` (`KismetMathLibrary.MakeVector` (.x (.location _returnvalue)) (.y (.location _returnvalue))) (.rotation _returnvalue) (.scale _returnvalue)) "Undefined" "OverrideRootScale" null null))
      (set `self.DeadBody` _returnvalue_2)
      (bind (_direction _switchcamera) (`Timeline|Timeline_3`)
        (:`Update`
          (`SceneComponent.K2_SetRelativeLocationAndRotation` (`self.FirstPersonCameraComponent`) _switchcamera (struct :`Pitch` -50.0) false false))))))

(event `InputAction|Pickup`
  (params (Key :type "Key Structure"))
  (bind _pickupitem (`self.pickupItem`))
  (bind _looking_at_actor (`self.Looking at Actor`))
  (bind _asrotdplayer_controller_bp (cast `/Game/ROTD/Blueprint/ROTDPlayerController_BP` (`GameplayStatics.GetPlayerController` 0) :!pure true))
  (bind _itemtype (`/Game/ROTD/Blueprint/PickupItems/ItemBase.ItemType` _pickupitem))
  (:`Pressed`
    (if (`KismetSystemLibrary.IsValid` _looking_at_actor)
      (bind _asitem_base (cast `/Game/ROTD/Blueprint/PickupItems/ItemBase` _looking_at_actor))
      (set `self.pickupItem` _asitem_base)
      (if (`SceneComponent.IsVisible` (`/Game/ROTD/Blueprint/PickupItems/ItemBase.InteractWidget` _asitem_base))
        (bind _asshooting_hud (cast `ShootingHUD` (`PlayerController.GetHUD` _asrotdplayer_controller_bp)))
        (`ShootingHUD.CanDisplayInteractItemInfo` _asshooting_hud false)
        (if (== (`/Game/ROTD/Blueprint/PickupItems/ItemBase.ClassName` _pickupitem) "/Game/ROTD/Blueprint/PickupItems/Item_Flashlight.Item_Flashlight_C")
          (`self.EquipFlashlight`)
          (else
            (`ROTDPlayerController.AddInventoryItem` _asrotdplayer_controller_bp _itemtype (`ROTDItems.Count` _itemtype) true)
            (`self.K2_DestroyActor` (`self.Looking at Actor`))))))))

(event `EquipFlashlight`
  ;[1 1 1] EquipFlashlight
  (bind _asitem_flashlight (cast `/Game/ROTD/Blueprint/PickupItems/Item_Flashlight` (`self.pickupItem`)))
  (set `self.Flashlight` _asitem_flashlight)
  (set `self.HasFlashlight` true)
  (`SceneComponent.K2_AttachToComponent` (`/Game/ROTD/Blueprint/PickupItems/ItemBase.ItemMesh` _asitem_flashlight) (`WeaponPickup.FP_Gun` (`self.CurrentWeapon`)) "Flashlight" "SnapToTarget" "SnapToTarget" "SnapToTarget" true))

(event `InputAction|TurnOnOff`
  (params (Key :type "Key Structure"))
  ;[1 1 1] EquipFlashlight
  (:`Pressed`
    (if (`self.HasFlashlight`)
      (`/Game/ROTD/Blueprint/PickupItems/Item_Flashlight.TurnOnFlashlight` (`self.Flashlight`)))))

(event `InputAction|WeaponChange`
  (params (Key :type "Key Structure"))
  (bind _currentweapon (`self.CurrentWeapon`))
  ;[1 1 1] Weapon change
  (:`Pressed`
    (if (`KismetSystemLibrary.IsValid` _currentweapon)
      (`self.SwitchWeapons` (`WeaponPickup.WeaponType` _currentweapon)))))

(event `InputAction|DropWeapon`
  (params (Key :type "Key Structure"))
  (bind _returnvalue (`KismetMathLibrary.RandomFloatInRange` -180.0 180.0))
  (bind _currentweapon (`self.CurrentWeapon`))
  (bind (_returnvalue_location _returnvalue_rotation _returnvalue_scale) (`KismetMathLibrary.BreakTransform` (`SceneComponent.K2_GetComponentToWorld` (`self.ThrowPoint`))))
  ;[1 1 1] Drop weapon
  (:`Pressed`
    (if (`KismetSystemLibrary.IsValid` _currentweapon)
      (bind _returnvalue_2 (`|SpawnActorFromClass` (`PickUpItemBase.ItemActor` _currentweapon) (`KismetMathLibrary.MakeTransform` _returnvalue_location (`KismetMathLibrary.MakeRotator` _returnvalue _returnvalue _returnvalue) _returnvalue_scale) "Undefined" "OverrideRootScale" null null))
      (bind _asitem_base (cast `/Game/ROTD/Blueprint/PickupItems/ItemBase` _returnvalue_2))
      (`/Game/ROTD/Blueprint/PickupItems/ItemBase.Push Pick Up Item Away` _asitem_base)
      (`self.DropWeaponAndSwitchWeapon`))))

(event `InputAction|Treatment`
  (params (Key :type "Key Structure"))
  ;[1 1 1] Treat
  (:`Pressed`
    (`self.TreatSelf` "EW_Hands")))

(event `InputAction|Use`
  (params (Key :type "Key Structure"))
  (bind _looking_at_actor (`self.Looking at Actor`))
  (:`Pressed`
    (if (`KismetSystemLibrary.IsValid` _looking_at_actor)
      (bind _interactivetype (message `/Game/ROTD/Blueprint/ItemInteractInterface_BP.GetItemType` _looking_at_actor))
      (if (`|EnumEquality` _interactivetype "NewEnumerator1")
        (message `/Game/ROTD/Blueprint/ItemInteractInterface_BP.Use` (`self.Looking at Actor`))))))

(fn `Can Display Interact Tips`
  (params (LookAtActor :type "Actor Object Reference"))
  (returns (Result :type Boolean))
  (if (`KismetSystemLibrary.DoesImplementInterface` LookAtActor "/Game/ROTD/Blueprint/ItemInteractInterface_BP.ItemInteractInterface_BP_C")
    (return true)
    (else
      (return false))))

(fn `Display InteractUI`
  (params (ItemName :type String)))

(fn `EyeSightLineTrace`
  (returns (IsHit :type Boolean) (HitActor :type "Actor Object Reference"))
  (bind _firstpersoncameracomponent (`self.FirstPersonCameraComponent`))
  (bind _returnvalue (`SceneComponent.K2_GetComponentLocation` _firstpersoncameracomponent))
  (bind (_outhit _returnvalue_2) (`KismetSystemLibrary.LineTraceSingle` _returnvalue (+ _returnvalue (* (`SceneComponent.GetForwardVector` _firstpersoncameracomponent) 400.0)) "TraceTypeQuery1"))
  (if _returnvalue_2
    (return true (`.HitActor` (`GameplayStatics.BreakHitResult` _outhit)))
    (else
      (return false null))))

(fn `GetItemInfo`
  (params (Tag :type String))
  (returns (Name :type String) (Detail :type String) (Num :type Integer64))
  (bind _returnvalue (`|GetDataTableRow` "/Game/ROTD/Data/SupplyItemDataTable.SupplyItemDataTable" (`KismetStringLibrary.Conv_StringToName` Tag))
    (:`then`
      (return (`.ItemName_5_C2438DA3459E36FE4E921CA00BF064B3` (break `/Game/ROTD/Data/FPickupItem` _returnvalue)) (`.ItemDetail_7_56FF483447F5840BC219C0BE35D3EE03` (break `/Game/ROTD/Data/FPickupItem` _returnvalue)) (`.ItemNum_10_F7809C8F4BE0AEBE7FDE34B3683492D4` (break `/Game/ROTD/Data/FPickupItem` _returnvalue))))
    (:`RowNotFound`
      (`KismetSystemLibrary.PrintString` "Not found")
      (return "" "" 0))))

(fn `GetShootingHUD`
  (returns (Hud :type "ShootingHUD Object Reference"))
  (bind _asshooting_hud (cast `ShootingHUD` (`PlayerController.GetHUD` (`GameplayStatics.GetPlayerController` 0))))
  (return _asshooting_hud))

(fn `HideInteractiveInfo`
  (params (LookingAt :type "Actor Object Reference"))
  (if (`KismetSystemLibrary.IsValid` LookingAt)
    (bind _interactivetype (message `/Game/ROTD/Blueprint/ItemInteractInterface_BP.GetItemType` LookingAt))
    (switch `/Game/ROTD/Blueprint/TraceLineHitEnum` _interactivetype
      (:`NewEnumerator0`
        (bind _asitem_base (cast `/Game/ROTD/Blueprint/PickupItems/ItemBase` LookingAt))
        (`PrimitiveComponent.SetRenderCustomDepth` (`/Game/ROTD/Blueprint/PickupItems/ItemBase.ItemMesh` _asitem_base) false)
        (`SceneComponent.SetHiddenInGame` (`/Game/ROTD/Blueprint/PickupItems/ItemBase.InteractWidget` _asitem_base) true false)
        (bind _hud (`self.GetShootingHUD`))
        (`ShootingHUD.CanDisplayInteractItemInfo` _hud false))
      (:`NewEnumerator1`
        (bind _asbp_parent_door (cast `/Game/PostDistrict/Blueprints/Buildings/BP_Parent_Door` LookingAt))
        (`SceneComponent.SetHiddenInGame` (`/Game/PostDistrict/Blueprints/Buildings/BP_Parent_Door.Tip` _asbp_parent_door) true false)))))

(fn `PlayLowDownWeaponMontage`)

(fn `Set Interact System`
  (bind _returnvalue (`KismetSystemLibrary.K2_SetTimerDelegate` (`|CreateDelegate` :!event `OnInteractSystem`) 0.2 true))
  (set `self.InteractSystemTimer` _returnvalue))

(fn `Show Interactive Info`
  (params (LookingAt :type "Actor Object Reference"))
  (locals (NewLocalVar_0 :type "Actor Object Reference"))
  (bind _interactivetype (message `/Game/ROTD/Blueprint/ItemInteractInterface_BP.GetItemType` LookingAt))
  (switch `/Game/ROTD/Blueprint/TraceLineHitEnum` _interactivetype
    (:`NewEnumerator0`
      (bind _asitem_base (cast `/Game/ROTD/Blueprint/PickupItems/ItemBase` LookingAt))
      (bind _output_get (set `self.As Item Base` _asitem_base))
      (`SceneComponent.SetHiddenInGame` (`/Game/ROTD/Blueprint/PickupItems/ItemBase.InteractWidget` _output_get) false false)
      (bind _hud (`self.GetShootingHUD`))
      (`ShootingHUD.CanDisplayInteractItemInfo` _hud true)
      (bind _asitem_base_2 (cast `/Game/ROTD/Blueprint/PickupItems/ItemBase` (`self.As Item Base`)))
      (`PrimitiveComponent.SetRenderCustomDepth` (`/Game/ROTD/Blueprint/PickupItems/ItemBase.ItemMesh` _asitem_base_2) true)
      (bind _hud_2 (`self.GetShootingHUD`))
      (bind _itemtype (`/Game/ROTD/Blueprint/PickupItems/ItemBase.ItemType` _asitem_base_2))
      (`ShootingHUD.UpdateInteractItemInfo` _hud_2 (`KismetTextLibrary.Conv_TextToString` (`ROTDItems.ItemName` _itemtype)) (`KismetTextLibrary.Conv_TextToString` (`ROTDItems.ItemDescription` _itemtype)) (`ROTDItems.Count` _itemtype)))
    (:`NewEnumerator1`
      (bind _asbp_parent_door (cast `/Game/PostDistrict/Blueprints/Buildings/BP_Parent_Door` LookingAt))
      (`SceneComponent.SetHiddenInGame` (`/Game/PostDistrict/Blueprints/Buildings/BP_Parent_Door.Tip` _asbp_parent_door) false false))))

(fn `ShowInteractiveInfoDoor`)

(fn `ShowPressTip`
  (params (CanShow :type Boolean) (IsOpen :type Boolean))
  (if CanShow
    (bind _hud (`self.GetShootingHUD`))
    (`ShootingHUD.IsDoorOpen` _hud IsOpen)
    (else
      (bind _hud_2 (`self.GetShootingHUD`))
      (`ShootingHUD.CanDisplayPressTip` _hud_2 false))))

(fn `UserConstructionScript`)