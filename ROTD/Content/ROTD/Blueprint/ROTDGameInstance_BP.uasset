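; Game instance for ROTD that owns the game's pause toggle.
; GamePause flips a Pause flag: pausing creates a PauseMenu_WB in the viewport and shows the cursor, while resuming calls CloseOptionScreen on that widget and hides the cursor.
; Both branches set Game and UI input mode on the ROTD player controller.
; The begin and end loading screen events only forward to the parent class.
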(event `self.BeginLoadingScreen`
  (params (MapName :type String))
  (`parent.BeginLoadingScreen` MapName))

(event `self.EndLoadingScreen`
  (params (InLoadWorld :type "World Object Reference"))
  (`parent.EndLoadingScreen` InLoadWorld))

(event `GamePause`
  (bind _asrotdplayer_controller_bp (cast `/Game/ROTD/Blueprint/ROTDPlayerController_BP` (`GameplayStatics.GetPlayerController` 0) :!pure true))
  (bind _asrotdplayer_controller_bp_2 (cast `/Game/ROTD/Blueprint/ROTDPlayerController_BP` (`GameplayStatics.GetPlayerController` 0) :!pure true))
  ;[1 1 1] Pause
  (if (`self.pause`)
    (`GameplayStatics.SetGamePaused` false)
    (`/Game/ROTD/UI/PauseMenu_WB.CloseOptionScreen` (stale _returnvalue))
    (set `self.pause` false)
    (`WidgetBlueprintLibrary.SetInputMode_GameAndUIEx` _asrotdplayer_controller_bp null)
    (set `PlayerController.bShowMouseCursor` false _asrotdplayer_controller_bp)
    (else
      (bind _asrotdplayer_controller_bp_3 (cast `/Game/ROTD/Blueprint/ROTDPlayerController_BP` (`GameplayStatics.GetPlayerController` 0)))
      (bind _returnvalue (`|CreateWidget` "/Game/ROTD/UI/PauseMenu_WB.PauseMenu_WB_C" _asrotdplayer_controller_bp_3))
      (`UserWidget.AddToViewport` _returnvalue 0)
      (`GameplayStatics.SetGamePaused` true)
      (set `self.pause` true)
      (`WidgetBlueprintLibrary.SetInputMode_GameAndUIEx` _asrotdplayer_controller_bp_2 null)
      (set `PlayerController.bShowMouseCursor` true _asrotdplayer_controller_bp_2))))