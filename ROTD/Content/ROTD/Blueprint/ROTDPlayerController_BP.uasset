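; Player controller for ROTD that handles pause, the inventory screen and skippable cutscenes.
; Pause closes an open inventory, otherwise calls the game instance's GamePause.
; The inventory toggle lazily creates and reuses one widget, reloads it from the controller's inventory data, and switches input mode and cursor.
; Cutscenes show a skip widget; Enter or sequence completion feeds one DoOnce path that stops playback, removes the widget and shows the ShootingHUD.
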(event `InputAction|PauseGame`
  (params (Key :type "Key Structure"))
  (bind _asrotdplayer_controller_bp (cast `/Game/ROTD/Blueprint/ROTDPlayerController_BP` (`GameplayStatics.GetPlayerController` 0) :!pure true))
  ;[1 1 1] Pause
  (:`Pressed`
    (if (`self.InventoryIsOpen`)
      (`Widget.RemoveFromParent` (`self.InventoryWB`))
      (set `self.InventoryIsOpen` false)
      (`WidgetBlueprintLibrary.SetInputMode_GameAndUIEx` _asrotdplayer_controller_bp null)
      (set `PlayerController.bShowMouseCursor` false _asrotdplayer_controller_bp)
      (else
        (bind _asrotdgame_instance_bp (cast `/Game/ROTD/Blueprint/ROTDGameInstance_BP` (`GameplayStatics.GetGameInstance`)))
        (`/Game/ROTD/Blueprint/ROTDGameInstance_BP.GamePause` _asrotdgame_instance_bp)))))

(event `PlaySkippableCutSense`
  (params (SequencePlayer :type "MovieSceneSequencePlayer Object Reference"))
  ;[1 1 1] CutScene
  (bind _output_get (set `self.Sequence Player` SequencePlayer))
  (`MovieSceneSequencePlayer.Play` _output_get)
  (add `MovieSceneSequencePlayer.OnFinished` _output_get (delegate `StopPlaySkippableCutscene`))
  (bind _returnvalue (`|CreateWidget` "/Game/ROTD/UI/SkipIntro_WB.SkipIntro_WB_C" self))
  (`UserWidget.AddToViewport` _returnvalue 0))

(event `StopPlaySkippableCutscene`
  ;[1 1 1] CutScene
  (`/Engine/EditorBlueprintResources/StandardMacros.DoOnce` false :!label _label
    (:`Completed`
      (`MovieSceneSequencePlayer.Stop` (`self.Sequence Player`))
      (bind _asshooting_hud (cast `ShootingHUD` (`self.GetHUD`)))
      (`ShootingHUD.ShowROTDHUD` _asshooting_hud true)
      (`Widget.RemoveFromParent` (stale `PlaySkippableCutSense` _returnvalue)))))

(event `Key|Enter`
  (params (Key :type "Key Structure"))
  ;[1 1 1] CutScene
  (:`Pressed`
    (goto _label)))

(event `InventoryOpenAndClose`
  (bind _asrotdplayer_controller_bp (cast `/Game/ROTD/Blueprint/ROTDPlayerController_BP` (`GameplayStatics.GetPlayerController` 0) :!pure true))
  (bind _asrotdplayer_controller_bp_2 (cast `/Game/ROTD/Blueprint/ROTDPlayerController_BP` (`GameplayStatics.GetPlayerController` 0) :!pure true))
  (bind _asrotdplayer_controller_bp_3 (cast `/Game/ROTD/Blueprint/ROTDPlayerController_BP` (`GameplayStatics.GetPlayerController` 0) :!pure true))
  ;[1 1 1] InventoryUI
  (if (`self.InventoryIsOpen`)
    (`Widget.RemoveFromParent` (`self.InventoryWB`))
    (set `self.InventoryIsOpen` false)
    (`WidgetBlueprintLibrary.SetInputMode_GameOnly` _asrotdplayer_controller_bp_2)
    (set `PlayerController.bShowMouseCursor` false _asrotdplayer_controller_bp_2)
    (else
      (set `self.InventoryIsOpen` true)
      (if (not (`KismetSystemLibrary.IsValid` (`self.InventoryWB`)))
        (bind _returnvalue (`|CreateWidget` "/Game/ROTD/UI/Inventory_WB.Inventory_WB_C"))
        (bind _output_get (set `self.InventoryWB` _returnvalue)))
      (`UserWidget.AddToViewport` _output_get 0)
      (`ROTDInventoryUI.ReloadInventory` (`self.InventoryWB`) (`ROTDPlayerController.InventoryItems` _asrotdplayer_controller_bp_3) (`ROTDPlayerController.InventoryData` _asrotdplayer_controller_bp_3))
      (`WidgetBlueprintLibrary.SetInputMode_GameAndUIEx` _asrotdplayer_controller_bp null)
      (set `PlayerController.bShowMouseCursor` true _asrotdplayer_controller_bp))))

(event `InputAction|InventoryOpenClose`
  (params (Key :type "Key Structure"))
  ;[1 1 1] InventoryUI
  (:`Pressed`
    (`self.InventoryOpenAndClose`)))

(fn `Show HUD`
  (bind _asshooting_hud (cast `ShootingHUD` (`self.GetHUD`)))
  (`ShootingHUD.ShowROTDHUD` _asshooting_hud true))

(fn `UserConstructionScript`)