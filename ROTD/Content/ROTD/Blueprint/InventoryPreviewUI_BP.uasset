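; InventoryPreviewUI_BP is an actor that renders a character's equipment for an inventory preview through a SceneCaptureComponent2D.
; The construction script restricts the capture to this actor's own components with ShowOnlyActorComponents, keeping the surrounding world out of the image.
; Setter functions swap the static meshes on the Helmet, Boot, Armor, Trousers and Clothing components to change the previewed gear.
; The event graph holds no logic.
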(fn `Set Armor`
  (params (NewMesh :type "StaticMesh Object Reference"))
  (`StaticMeshComponent.SetStaticMesh` (`self.Armor`) NewMesh))

(fn `Set Boot`
  (params (NewMesh :type "StaticMesh Object Reference"))
  (`StaticMeshComponent.SetStaticMesh` (`self.Boot`) NewMesh))

(fn `Set Clothing`
  (params (NewMesh :type "StaticMesh Object Reference"))
  (`StaticMeshComponent.SetStaticMesh` (`self.Clothing`) NewMesh))

(fn `Set Trousers`
  (params (NewMesh :type "StaticMesh Object Reference"))
  (`StaticMeshComponent.SetStaticMesh` (`self.Trousers`) NewMesh))

(fn `SetHelmet`
  (params (NewMesh :type "StaticMesh Object Reference"))
  (`StaticMeshComponent.SetStaticMesh` (`self.Helmet`) NewMesh))

(fn `UserConstructionScript`
  (`SceneCaptureComponent.ShowOnlyActorComponents` (`self.SceneCaptureComponent2D`) self false))