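; Flashlight pickup item that provides a switchable spot light.
; TurnOnFlashlight acts as a toggle, using a FlipFlop to alternately show and hide the SpotLight, starting with show.
; GetItemType reports a fixed item-type enum value, while the Use event is an empty stub.
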(event `/Game/ROTD/Blueprint/ItemInteractInterface_BP.Use`)

(event `TurnOnFlashlight`
  (bind _spotlight (`self.SpotLight`))
  (`/Engine/EditorBlueprintResources/StandardMacros.FlipFlop`
    (:`A`
      (`SceneComponent.SetVisibility` _spotlight true false))
    (:`B`
      (`SceneComponent.SetVisibility` _spotlight false false))))

(fn `GetItemType`
  (returns (InteractiveType :type "/Game/ROTD/Blueprint/TraceLineHitEnum Enum"))
  (return "NewEnumerator0"))

(fn `UserConstructionScript`
  (`parent.UserConstructionScript`))