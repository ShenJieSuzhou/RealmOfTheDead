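; ROTDGameMode_BP is the ROTD game mode that opens a level with a skippable cutscene.
; On BeginPlay it passes the first LevelSequenceActor's player to ROTDPlayerController_BP for playback, or calls StartGame if the level has none.
; StartGame is a stub holding only a short delay, and the zombie spawn event only prints a message and is not called within this graph.
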(event `self.ReceiveBeginPlay`
  (`self.PlayCutSenses`))

(event `PlayCutSenses`
  ;[1 1 1] Play Cutsence logic
  (bind _outactors (`GameplayStatics.GetAllActorsOfClass` "/Script/LevelSequence.LevelSequenceActor"))
  (if (`KismetArrayLibrary.Array_IsValidIndex` _outactors)
    (`/Game/ROTD/Blueprint/ROTDPlayerController_BP.PlaySkippableCutSense` (cast `/Game/ROTD/Blueprint/ROTDPlayerController_BP` (`GameplayStatics.GetPlayerController` 0) :!pure true) (`LevelSequenceActor.SequencePlayer` (`|GetArrayItem` _outactors)))
    (else
      (`self.Start Game`))))

(event `Start Game`
  ;[1 1 1] Start Game
  (`KismetSystemLibrary.Delay` 1.0))

(event `Spawn Zombiles`
  ;[1 1 1] Zombie Spawn
  (`KismetSystemLibrary.PrintString` "Spawn Zombies"))

(fn `UserConstructionScript`)