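; ROTDEntryMode_BP is the entry mode Blueprint that brings up the main menu.
; On BeginPlay it creates and stores a Menus_WB widget, adds it to the viewport, and enables game-and-UI input with a visible cursor.
; StartLoadResource hides the menu's loading view and enables the start button.
; AssetsLoadComplete is empty, and the PreLoadMaterials call is never executed.
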(event `self.ReceiveBeginPlay`
  (bind _returnvalue (`GameplayStatics.GetPlayerController` 0))
  (bind _returnvalue_2 (`|CreateWidget` "/Game/ROTD/UI/Menus_WB.Menus_WB_C"))
  (bind _output_get (set `self.Mainmenu` _returnvalue_2))
  (`UserWidget.AddToViewport` _output_get 0)
  (`WidgetBlueprintLibrary.SetInputMode_GameAndUIEx` _returnvalue null)
  (set `PlayerController.bShowMouseCursor` true _returnvalue))

(event `StartLoadResource`
  (`Widget.SetVisibility` (`/Game/ROTD/UI/Menus_WB.LoadingView` (`self.Mainmenu`)) "Hidden")
  (`Widget.SetIsEnabled` (`/Game/ROTD/UI/Menus_WB.StartBtn` (`self.Mainmenu`)) true))

(event `self.AssetsLoadComplete`)

(fn `UserConstructionScript`)