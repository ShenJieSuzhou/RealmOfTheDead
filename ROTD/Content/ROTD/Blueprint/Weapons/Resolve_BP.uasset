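; Resolve_BP is a weapon Blueprint for the player's Henry_BP character, with only aim-down-sights implemented.
; It caches the player character on BeginPlay, then its ADS and recover events each play a timeline that lerps the first-person camera FOV and Mesh1P position while setting a fixed mesh rotation.
; Fire, reload and shell-drop events are empty, and both ammo functions simply return false.
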(event `self.ReceiveBeginPlay`
  (bind _ashenry_bp (cast `/Game/ROTD/Blueprint/Henry_BP` (`GameplayStatics.GetPlayerCharacter` 0)))
  (set `self.As Henry BP` _ashenry_bp))

(event `self.WeaponFire`)

(event `self.WeaponReload`)

(event `self.BulletShellDrop`)

(event `self.WeaponADS`
  ;[1 1 1] ADS
  (bind (_direction _float) (`Timeline|Timeline_0` :!via `PlayFromStart`)
    (:`Update`
      (set `self.ADSDistance` 60.0)
      (`CameraComponent.SetFieldOfView` (`ROTDCharacter.FirstPersonCameraComponent` (`self.As Henry BP`)) (`KismetMathLibrary.Lerp` 90.0 (`self.ADSDistance`) _float))
      (`SceneComponent.K2_SetRelativeTransform` (`ROTDCharacter.Mesh1P` (`self.As Henry BP`)) (`KismetMathLibrary.MakeTransform` (`KismetMathLibrary.VLerp` (3.177 -1.02 -23.0) (3.177 0.0 -16.0) _float) (struct :`Yaw` -1.0)) false false))))

(event `self.WeaponRecoverADS`
  ;[1 1 1] ADS
  (bind (_direction _float) (`Timeline|Timeline_1` :!via `PlayFromStart`)
    (:`Update`
      (`CameraComponent.SetFieldOfView` (`ROTDCharacter.FirstPersonCameraComponent` (`self.As Henry BP`)) (`KismetMathLibrary.Lerp` (`self.ADSDistance`) 90.0 _float))
      (`SceneComponent.K2_SetRelativeTransform` (`ROTDCharacter.Mesh1P` (`self.As Henry BP`)) (`KismetMathLibrary.MakeTransform` (`KismetMathLibrary.VLerp` (3.177 -0.0 -16.0) (3.177 -1.02 -23.0) _float) (struct :`Yaw` 4.0)) false false))))

(fn `AmmoCheck`
  (returns (NewParam :type Boolean))
  (return false))

(fn `AmmoReload`
  (returns (Result :type Boolean))
  (return false))

(fn `UserConstructionScript`)