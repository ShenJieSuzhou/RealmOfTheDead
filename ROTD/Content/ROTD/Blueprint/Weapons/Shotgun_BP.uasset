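; Shotgun weapon Blueprint whose graphs handle only the ejection of spent shell casings; no firing logic is present here.
; BulletShellDrop calls ShellDrop to spawn a RifleBS_BP casing at the gun's ShellEjection socket and launch it with a physics impulse along its local axes.
; After a short delay it plays a casing sound at the player's location, then destroys the shell several seconds later.
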(event `self.BulletShellDrop`
  (bind _output (`self.ShellDrop` (`self.FP_Gun`) "ShellEjection" "/Game/ROTD/Blueprint/Weapons/RifleBS_BP.RifleBS_BP_C" -60.0))
  (`KismetSystemLibrary.Delay` 1.0)
  (`GameplayStatics.PlaySoundAtLocation` "/Game/ROTD/Sounds/Bullets/Bullets-shell-casings-607.Bullets-shell-casings-607" (`self.K2_GetActorLocation` (`GameplayStatics.GetPlayerCharacter` 0)) (struct) 1.0 1.0 0.0 null null null null)
  (`KismetSystemLibrary.Delay` 10.0)
  (`self.K2_DestroyActor` _output))

(fn `ShellDrop`
  (params (Weapon :type "SceneComponent Object Reference") (InSocketName :type Name) (Class :type "Actor Class Reference") (Speed :type "Float (double-precision)") (Up :type "Float (double-precision)") (back :type "Float (double-precision)"))
  (returns (output :type "/Game/ROTD/Blueprint/Weapons/RifleBS_BP Object Reference"))
  (bind _returnvalue (`|SpawnActorFromClass` Class (`SceneComponent.GetSocketTransform` Weapon InSocketName "RTS_World") "AlwaysSpawn" "OverrideRootScale" null null))
  (bind _asrifle_bs_bp (cast `/Game/ROTD/Blueprint/Weapons/RifleBS_BP` _returnvalue))
  (bind _shell (`/Game/ROTD/Blueprint/Weapons/RifleBS_BP.Shell` _asrifle_bs_bp))
  (`PrimitiveComponent.SetSimulatePhysics` _shell true)
  (`PrimitiveComponent.AddImpulse` _shell (+ (* (`SceneComponent.GetUpVector` _shell) back) (* (`SceneComponent.GetRightVector` _shell) Speed) (* (`SceneComponent.GetForwardVector` _shell) Up)) "None" false)
  (return _asrifle_bs_bp))

(fn `UserConstructionScript`)